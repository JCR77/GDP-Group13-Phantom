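; Sniper rifle weapon Blueprint that extends a parent weapon with a fire animation and a scoped aim view.
; Firing runs the parent logic, then plays the rifle's animation on the gun mesh.
; Aiming as the current weapon blocks switching and reloading, then after a brief delay shows the scope widget and hides the gun and player pawn, if the widget is not already shown.
; Exiting aim reverses these changes.
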(event EventWeaponFire
  (params (IsAI :type Boolean) (ShooterPawnReference :type Pawn%20Object%20Reference) (FireType :type FireType%20Enum :default "NewEnumerator0"))
  (|CallParentFunction IsAI ShooterPawnReference FireType)
  (Components|Animation|PlayAnimation (Variables|Default|GetGunMesh) "/Game/MilitaryWeapDark/Weapons/Anims/Fire_SniperRifle_W.Fire_SniperRifle_W" false))

(event EventOnAimEnter
  (bind _playerreference (Variables|Default|GetPlayerReference))
  (bind _playerreference_2 (Variables|Default|GetPlayerReference))
  (bind _sniperscopewidget (Variables|/Game/Blueprints/FPCharacter.FPCharacter_C|GetSniperScopeWidget _playerreference))
  (|CallParentFunction)
  (if (== (Variables|/Game/Blueprints/FPCharacter.FPCharacter_C|GetCurrentWeapon (Variables|Default|GetPlayerReference)) self)
    (Variables|/Game/Blueprints/FPCharacter.FPCharacter_C|SetCanSwitchWeapon _playerreference_2 false)
    (Variables|/Game/Blueprints/FPCharacter.FPCharacter_C|SetCanReload _playerreference_2 false)
    (Utilities|FlowControl|Delay 0.1)
    (if (not (UserInterface|Viewport|IsinViewport _sniperscopewidget))
      (UserInterface|Viewport|AddtoViewport _sniperscopewidget 0)
      (Development|SetHiddeninGame (Variables|Default|GetGunMesh) true false)
      (Rendering|SetActorHiddenInGame (Game|Player|GetPlayerPawn 0) true))))

(event EventOnAimExit
  (bind _playerreference (Variables|Default|GetPlayerReference))
  (|CallParentFunction)
  (Variables|/Game/Blueprints/FPCharacter.FPCharacter_C|SetCanSwitchWeapon _playerreference true)
  (Variables|/Game/Blueprints/FPCharacter.FPCharacter_C|SetCanReload _playerreference true)
  (Widget|RemovefromParent (Variables|/Game/Blueprints/FPCharacter.FPCharacter_C|GetSniperScopeWidget _playerreference))
  (Development|SetHiddeninGame (Variables|Default|GetGunMesh) false false)
  (Rendering|SetActorHiddenInGame (Game|Player|GetPlayerPawn 0) false))

(fn ConstructionScript
  (|CallParentFunction))