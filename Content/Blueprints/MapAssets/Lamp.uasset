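; Lamp actor with a spotlight that tests the player's distance as a debug-only hidden check.
; BeginPlay caches the player pawn as an FPCharacter reference.
; Every Tick prints the spotlight-to-player distance, then "hidden" within a fixed radius or "Not Hidden" beyond it.
; The Sphere overlap event is empty, so detection relies solely on distance polling and changes no state.
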(event OnComponentBeginOverlap(Sphere)
  (params (OverlappedComponent :type Primitive%20Component%20Object%20Reference) (OtherActor :type Actor%20Object%20Reference) (OtherComp :type Primitive%20Component%20Object%20Reference) (OtherBodyIndex :type Integer) (bFromSweep :type Boolean) (SweepResult :type Hit%20Result%20Structure%20%28by%20ref%29)))

(event EventBeginPlay
  (bind _asfpcharacter (Utilities|Casting|CastToFPCharacter (Game|Player|GetPlayerPawn 0)))
  (Variables|Default|SetPlayerCharRef _asfpcharacter))

(event Collision|EventActorBeginOverlap
  (params (OtherActor :type Actor%20Object%20Reference)))

(event EventTick
  (params (DeltaSeconds :type Float%20%28single-precision%29))
  (bind _spotlight (Variables|Default|GetSpotLight))
  (bind _playercharref (Variables|Default|GetPlayerCharRef))
  (bind _returnvalue (Transformation|GetWorldLocation _spotlight))
  (bind _rootcomponent (Variables|/Script/Engine.Actor|GetRootComponent _playercharref))
  (bind _returnvalue_2 (Transformation|GetWorldLocation _rootcomponent))
  (bind _returnvalue_3 (Math|Vector|Distance(Vector) _returnvalue _returnvalue_2))
  (Development|PrintString (Utilities|String|ToString(Float) _returnvalue_3) true true "(R=0.000000,G=0.660000,B=1.000000,A=1.000000)" 0.0)
  (if (<= _returnvalue_3 6e+02)
    (Development|PrintString "hidden" true true "(R=0.000000,G=0.660000,B=1.000000,A=1.000000)" 0.0)
    (else
      (Development|PrintString "Not Hidden" true true "(R=0.000000,G=0.660000,B=1.000000,A=1.000000)" 0.0))))

(fn ConstructionScript)