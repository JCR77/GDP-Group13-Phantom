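; Shotgun weapon Blueprint that extends a parent weapon class with shotgun-specific firing effects and reload timing.
; WeaponFire runs the parent fire logic, then plays the shotgun fire animation on the gun mesh and spawns a shell particle at its AmmoEject socket.
; SetReloadTime scales the reload duration with magazine capacity.
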(event Custom|Set%20Reload%20Time
  (Variables|Default|SetReloadTime (* (Variables|Default|GetMaxMagAmmo) 0.5))
  (CallFunction|SetReloadTime))

(event EventBeginPlay
  (|CallParentFunction))

(event Collision|EventActorBeginOverlap
  (params (OtherActor :type Actor%20Object%20Reference))
  (|CallParentFunction OtherActor) ; This node is disabled and will not be called.\nDrag off pins to build functionality.
)

(event EventTick
  (params (DeltaSeconds :type Float%20%28single-precision%29))
  (|CallParentFunction DeltaSeconds) ; This node is disabled and will not be called.\nDrag off pins to build functionality.
)

(event EventWeaponFire
  (params (IsAI :type Boolean) (ShooterPawnReference :type Pawn%20Object%20Reference) (FireType :type FireType%20Enum :default "NewEnumerator0"))
  (bind _gunmesh (Variables|Default|GetGunMesh))
  (bind _returnvalue (Transformation|GetSocketTransform _gunmesh "AmmoEject" "RTS_World"))
  (|CallParentFunction IsAI ShooterPawnReference FireType)
  (Components|Animation|PlayAnimation _gunmesh "/Game/MilitaryWeapDark/Weapons/Anims/Fire_Shotgun_W.Fire_Shotgun_W" false)
  (Effects|SpawnEmitteratLocation "/Game/Particles/FXShotgunShell.FXShotgunShell" (.location _returnvalue) (.rotation _returnvalue)))

(fn ConstructionScript
  (|CallParentFunction))