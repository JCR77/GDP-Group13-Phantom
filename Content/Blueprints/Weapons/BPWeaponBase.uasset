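; Base weapon Blueprint handling hitscan firing, ammo and reloading for the FPCharacter player.
; WeaponFire spends a round, traces from the camera with random BulletSpread, spawns an impact effect and sends TakeDamageMessage to the hit actor.
; The trace hits only WorldStatic and WorldDynamic objects; the muzzle socket is passed but unused.
; Reload refills from total ammo, discarding rounds left in the magazine; ammo checks are separate, not enforced by WeaponFire.
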(event EventBeginPlay
  (bind _asfpcharacter (Utilities|Casting|CastToFPCharacter (Game|Player|GetPlayerPawn 0)))
  (Variables|Default|SetPlayerReference _asfpcharacter))

(event Collision|EventActorBeginOverlap
  (params (OtherActor :type Actor%20Object%20Reference)))

(event EventTick
  (params (DeltaSeconds :type Float%20%28single-precision%29)))

(fn ConstructionScript)

(fn WeaponFire
  (Variables|Ammo|SetCurrentAmmo (- (Variables|Ammo|GetCurrentAmmo) 1))
  (bind _hitresult (CallFunction|CalculateShot (Variables|/Game/Blueprints/FPCharacter.FPCharacter_C|GetCamera (Variables|Default|GetPlayerReference)) (Variables|Default|GetGunMesh) "MuzzleFlash"))
  (Game|SpawnActorfromClass (Variables|Default|GetImpactEffectClass) (Math|Transform|MakeTransform (.ImpactPoint (Collision|BreakHitResult _hitresult)) "0, 0, 0" "1,1,1") "Undefined" 0 _hitresult (.bBlockingHit (Collision|BreakHitResult _hitresult)) 0)
  (CallFunction|AddDamage _hitresult))

(fn WeaponReload
  (Variables|Ammo|SetCurrentAmmo (Math|Integer|Min(Integer) (Variables|Ammo|GetMaxMagAmmo) (Variables|Ammo|GetCurrentTotalAmmo)))
  (Variables|Ammo|SetCurrentTotalAmmo (- (Variables|Ammo|GetCurrentTotalAmmo) (Math|Integer|Min(Integer) (Variables|Ammo|GetMaxMagAmmo) (Variables|Ammo|GetCurrentTotalAmmo)))))

(fn CheckAmmoinMag
  (return (> (Variables|Ammo|GetCurrentAmmo) 0) (== (Variables|Ammo|GetCurrentAmmo) (Variables|Ammo|GetMaxMagAmmo))))

(fn CheckAmmo
  (return (> (Variables|Ammo|GetCurrentTotalAmmo) 0)))

(fn CalculateShot
  (params (Camera :type Camera%20Component%20Object%20Reference) (WeaponMesh :type Scene%20Component%20Object%20Reference) (WeaponFireSocket :type Name))
  (bind _bulletspread (Variables|Default|GetBulletSpread))
  (bind _returnvalue (* _bulletspread -1.0))
  (Utilities|FlowControl|Sequence
    (:then_0
      (Variables|Default|SetLocal%20Camera Camera)
      (LocalVariables|SetLocalWeaponMesh WeaponMesh)
      (LocalVariables|SetLocalSocketName WeaponFireSocket))
    (:then_1
      (bind _outhit (Collision|LineTraceForObjects (.location (Transformation|GetWorldTransform (Variables|Default|GetLocal%20Camera))) (Math|Vector|MakeVector (+ (.X (Math|Vector|BreakVector (+ (.location (Transformation|GetWorldTransform (Variables|Default|GetLocal%20Camera))) (* (Math|Vector|GetForwardVector (.rotation (Transformation|GetWorldTransform (Variables|Default|GetLocal%20Camera)))) 1e+04)))) (Math|Random|RandomFloatinRange _returnvalue _bulletspread)) (+ (.Y (Math|Vector|BreakVector (+ (.location (Transformation|GetWorldTransform (Variables|Default|GetLocal%20Camera))) (* (Math|Vector|GetForwardVector (.rotation (Transformation|GetWorldTransform (Variables|Default|GetLocal%20Camera)))) 1e+04)))) (Math|Random|RandomFloatinRange _returnvalue _bulletspread)) (+ (.Z (Math|Vector|BreakVector (+ (.location (Transformation|GetWorldTransform (Variables|Default|GetLocal%20Camera))) (* (Math|Vector|GetForwardVector (.rotation (Transformation|GetWorldTransform (Variables|Default|GetLocal%20Camera)))) 1e+04)))) (Math|Random|RandomFloatinRange _returnvalue _bulletspread))) (Utilities|Array|MakeArray "ObjectTypeQuery1" "ObjectTypeQuery2") false (Utilities|Array|MakeArray (Game|Player|GetPlayerPawn 0)) "None"))
      (return _outhit))))

(fn AddDamage
  (params (HitResult :type Hit%20Result%20Structure))
  (Class|TakeDamage|TakeDamage(Message) (.HitActor (Collision|BreakHitResult HitResult)) (Variables|Default|GetAmmoData) (Variables|Default|GetCriticalHitDamageModifier) HitResult))