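; A lamp actor that can be switched off by damage and tracks whether the player stands within its radius while lit.
; BeginPlay caches the FPCharacter pawn, and sphere overlaps set PlayerInside, only turning it true while the lamp is on.
; TakeDamage on a box component hides the spotlight and a mesh, then clears IsOn and PlayerInside, with no path to relight.
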(event OnComponentBeginOverlap(Sphere)
  (params (OverlappedComponent :type Primitive%20Component%20Object%20Reference) (OtherActor :type Actor%20Object%20Reference) (OtherComp :type Primitive%20Component%20Object%20Reference) (OtherBodyIndex :type Integer) (bFromSweep :type Boolean) (SweepResult :type Hit%20Result%20Structure%20%28by%20ref%29))
  (if (and (== OtherActor (Variables|Default|GetPlayerCharRef)) (Variables|Default|GetIsOn))
    (Variables|Default|SetPlayerInside true)))

(event OnComponentEndOverlap(Sphere)
  (params (OverlappedComponent :type Primitive%20Component%20Object%20Reference) (OtherActor :type Actor%20Object%20Reference) (OtherComp :type Primitive%20Component%20Object%20Reference) (OtherBodyIndex :type Integer))
  (if (== OtherActor (Variables|Default|GetPlayerCharRef))
    (Variables|Default|SetPlayerInside false)))

(event EventBeginPlay
  (bind _asfpcharacter (Utilities|Casting|CastToFPCharacter (Game|Player|GetPlayerPawn 0)))
  (Variables|Default|SetPlayerCharRef _asfpcharacter))

(event EventTakeDamage
  (params (AmmoData :type Ammo%20Data%20Structure) (CriticalHitModifier :type Float%20%28single-precision%29) (HitResult :type Hit%20Result%20Structure) (HitComponent :type Primitive%20Component%20Object%20Reference))
  (Utilities|Casting|CastToBoxComponent HitComponent)
  (Rendering|SetVisibility (Variables|Default|GetSpotLight) false false)
  (Variables|Default|SetIsOn false)
  (Variables|Default|SetPlayerInside false))

(fn ConstructionScript)